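; Blueprint Interface that exposes a fighting-game character's state to other Blueprints through read-only getter functions, with no logic of its own.
; Getters are grouped by domain: transform, player name, character setup, movement inputs, health, locomotion and fighting state.
; Each returns several values at once, covering details such as animation play rate, crouch, defend, knockdown, combo progress and match loss.
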(fn BaseData
  (return "0, 0, 0" "0, 0, 0"))

(fn PlayerData
  (return "None" 0))

(fn CharacterData
  (return "NewEnumerator0" 0 0 0 0 0 0.0 0.0))

(fn GetInputs
  (return 0.0 0.0 false))

(fn Health&Damage
  (return false 0))

(fn Locomotion
  (return false false false false 0.0))

(fn FightingData
  (return false false false "" false false "NewEnumerator3" 0 false false false))