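; Main game instance Blueprint that holds fight data and handles level changes, settings and confirmation prompts.
; StartFight optionally stores new FightingData, then opens its map through an enum-to-level select between main menu and forge test map.
; It creates the settings and selection message widgets; enum-coded Yes/No actions either dismiss the message or quit the game.
; Getter functions expose FightingData, while the other data getters are empty or return defaults.
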(event Custom|Start%20Fight
  (params (Set%20New%20Data :type Boolean) (Fighting%20Data :type S%20Fighting%20Data%20Structure))
  ;[1 1 1] Change FightingData
  (Utilities|FlowControl|Sequence
    (:then_0
      (if Set%20New%20Data
        (Variables|FightingData|SetFighting%20Data Fighting%20Data)))
    (:then_1
      (CallFunction|OpenLevel (Utilities|Struct|BreakS_Map_Data (Utilities|Struct|BreakS_Fighting_Data Fighting%20Data))))))

(event Custom|Open%20Level
  (params (Map :type E_Maps%20Enum :default "NewEnumerator0"))
  ;[1 1 1] Open Level
  (Game|OpenLevel(byObjectReference) (Utilities|Select :Index Map :NewEnumerator1 "/Game/Maps/L_MainMenu.L_MainMenu" :NewEnumerator0 "/Game/Maps/Test_Maps/L_Test_Map.L_Test_Map")))

(event Custom|Open%20Settings
  (params (OwningPlayer :type Player%20Controller%20Object%20Reference))
  ;[1 1 1] Open Settings
  (bind _returnvalue (UserInterface|CreateWidget "/Game/Blueprints/UI/Settings/WB_Settings.WB_Settings_C" OwningPlayer))
  (Variables|Settings|SetSettings%20Widget _returnvalue))

(event Custom|Create%20Selection%20Message
  (params (OwningPlayer :type Player%20Controller%20Object%20Reference) (Message :type Text) (Yes%20Function :type E_Message_Function%20Enum :default "NewEnumerator1") (No%20Function :type E_Message_Function%20Enum :default "NewEnumerator1"))
  ;[1 1 1] Selection Message
  ;;[1 1 1] Create Selection Message
  (bind _returnvalue (UserInterface|CreateWidget "/Game/Blueprints/UI/Custom/WB_SelectionMessage.WB_SelectionMessage_C" OwningPlayer Message Yes%20Function No%20Function))
  (bind _output_get (Variables|MessageWidget|SetSelection%20Message%20Widget _returnvalue))
  (UserInterface|Viewport|AddtoViewport _output_get 0))

(event Custom|Selection%20Message%20Function
  (params (Yes%20Selection :type Boolean) (Yes%20Function :type E_Message_Function%20Enum :default "NewEnumerator1") (No%20Function :type E_Message_Function%20Enum :default "NewEnumerator1"))
  ;[1 1 1] Selection Message
  ;;[1 1 1] Selection Message Function
  (if Yes%20Selection
    (switch Utilities|FlowControl|Switch|SwitchonE_Message_Function Yes%20Function
      (:NewEnumerator1
        (bind _selection_message_widget (Variables|MessageWidget|GetSelection%20Message%20Widget :!label _label)
          (:then
            (Widget|RemovefromParent _selection_message_widget))
          (:else)))
      (:NewEnumerator0
        (Game|QuitGame 0 "Quit" false :!label _label_2)))
    (else
      (switch Utilities|FlowControl|Switch|SwitchonE_Message_Function No%20Function
        (:NewEnumerator1
          (goto _label))
        (:NewEnumerator0
          (goto _label_2))))))

(fn GetGameRefs
  (return 0 0 0 0 0 0 0 0))

(fn GetGameInstanceData
  (return (Variables|FightingData|GetFighting%20Data)))

(fn GetGameModeData
  (return "" false 0 false))

(fn GetGameStateData
  (return ""))