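; Main game mode that runs the fight-start intro and holds the game-started flag and match timer.
; On BeginPlay it shows the WB_FightStart widget with a self reference and starts its animation; the animation-ended event sets GameStarted and removes the widget.
; SetTimer runs a macro that counts Timer down each second through a looping Delay.
; GetGameModeData exposes both values; the other getters are empty stubs.
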(event Custom|Fight%20UI%20Animation%20Ended
  ;[1 1 1] Fight UI Animation Ended
  (Variables|Gamedata|SetGame%20Started true)
  (bind _start_fight_widget (Variables|GameData|GetStart%20Fight%20Widget)
    (:then
      (Widget|RemovefromParent _start_fight_widget))
    (:else)))

(event Custom|Set%20Timer
  (params (Timer :type Integer))
  ;[1 1 1] Set Timer
  (Utilities|TimerMacro Timer))

(event EventBeginPlay
  ;[1 1 1] Begin Play
  (bind _returnvalue (UserInterface|CreateWidget "/Game/Blueprints/HUD-Widget/GamePlay/Custom/WB_FightStart.WB_FightStart_C" 0 self))
  (bind _output_get (Variables|GameData|SetStart%20Fight%20Widget _returnvalue))
  (UserInterface|Viewport|AddtoViewport _output_get 0)
  (Default|StartUIFightAnimation _output_get 3))

(fn ConstructionScript)

(fn GetGameRefs
  (return 0 0 0 0 0 0 0))

(fn GetGameModeData
  (return (Variables|Gamedata|GetGame%20Started) (Variables|GameData|GetTimer)))

(fn GetGameStateData
  (return ""))