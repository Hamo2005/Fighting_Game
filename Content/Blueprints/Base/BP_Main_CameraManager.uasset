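; Player camera manager that keeps the player and their enemy framed with a follow camera.
; Each tick it gets both characters through message calls, taking camera height from the player's Spine_02 socket.
; BlueprintUpdateCamera backs away from their midpoint along the player's forward vector by a clamped, separation-based distance.
; It smoothly interpolates location and yaw-only rotation toward that midpoint, with a fixed FOV.
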(event EventTick
  (params (DeltaSeconds :type Float%20%28single-precision%29))
  ;[1 1 1] Update
  (Base|GetRefs)
  (CallFunction|GetPlayerData)
  (CallFunction|GetEnemyData))

(fn ConstructionScript)

(fn BlueprintUpdateCamera
  (params (CameraTarget :type Actor%20Object%20Reference))
  (bind _returnvalue (Utilities|Time|GetWorldDeltaSeconds))
  (bind _enemy_location (Variables|BaseData|GetEnemy%20Location))
  (bind _camera_length (Variables|Data|GetCamera%20Length))
  (bind _player_location (Variables|BaseData|GetPlayer%20Location))
  (bind _z (Math|Vector|BreakVector _player_location))
  (bind _returnvalue_2 (Math|Vector|Distance(Vector) _player_location _enemy_location))
  (bind _returnvalue_3 (+ _player_location _enemy_location))
  (bind _returnvalue_4 (/ _returnvalue_3 2))
  (bind (_x _y) (Math|Vector|BreakVector _returnvalue_4))
  (bind _returnvalue_5 (Math|Vector|MakeVector _x _y _z))
  ;[1 1 1] Update Camera Location, Rotation & FOV
  (return (Math|Interpolation|VInterpTo (Camera|GetCameraLocation) (- _returnvalue_5 (* (Math|Vector|GetForwardVector (Variables|BaseData|GetPlayer%20Rotation)) (Math|Float|Clamp(Float) _returnvalue_2 (* _camera_length 2.0) (+ (/ _returnvalue_2 2.0) _camera_length)))) _returnvalue 1e+01) (Math|Interpolation|RInterpTo (Camera|GetCameraRotation) (Math|Rotator|MakeRotator 0.0 0.0 (.yaw (Math|Rotator|FindLookatRotation (Transformation|GetActorLocation) _returnvalue_5))) _returnvalue 1e+01) 9e+01 true))

(fn GetRefs
  ;[1 1 1] Get Refs
  (bind _asbp_player (Utilities|Casting|CastToBP_Player (Pawn|GetControlledPawn (Game|Player|GetOwningPlayerController))))
  (bind _output_get (Variables|Refs|SetPlayer _asbp_player))
  (bind (_game_instance _game_mode _game_state _player_controller _camera_manager _player_state _player _enemy) (Class|BPGameData|GetGameRefs(Message) _output_get))
  (Variables|Refs|SetPlayer%20Controller _player_controller)
  (Variables|Refs|SetEnemy _enemy))

(fn GetPlayerData
  ;[1 1 1] Get Player Data
  (bind _player (Variables|Refs|GetPlayer)
    (:then
      (bind (_actor_rotation _actor_location) (Class|BPCharacterData|BaseData(Message) _player))
      (Variables|BaseData|SetPlayer%20Rotation _actor_rotation)
      (Variables|BaseData|SetPlayer%20Location (Math|Vector|MakeVector (.X (Math|Vector|BreakVector _actor_location)) (.Y (Math|Vector|BreakVector _actor_location)) (.Z (Math|Vector|BreakVector (Transformation|GetSocketLocation (Variables|/Script/Engine.Character|GetMesh _player) "Spine_02"))))))
    (:else)))

(fn GetEnemyData
  ;[1 1 1] Get Enemy Data
  (bind _enemy (Variables|Refs|GetEnemy)
    (:then
      (bind _actor_location (Class|BPCharacterData|BaseData(Message) _enemy))
      (Variables|BaseData|SetEnemy%20Location _actor_location))
    (:else)))