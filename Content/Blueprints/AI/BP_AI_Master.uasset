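; BP_AI_Master is an AI-controlled fighter that picks attacks, blocks and jumps at random, using Hit and state flags not defined here.
; A looping timer fires AI_Hit, which acts only once GameStarted and then resets the timer with a new random interval.
; Each pass chooses a random hit type influenced by Combo, may briefly raise Defend and may call AIJump.
; Finish overrides the choice with a dedicated hit, also triggered every Tick while set.
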(event Custom|AI_Hit
  (bind _returnvalue (Math|Random|RandomFloatinRange 0.5 1.5))
  (if (Variables|Default|GetGame%20Started)
    (CallFunction|Hit (select (Variables|Default|GetFinish) "NewEnumerator3" (Utilities|Select :Index (Math|Random|RandomIntegerinRange 0 2) :Option%200 "NewEnumerator0" :Option%201 (select (Variables|Default|GetCombo) "NewEnumerator2" (select (Math|Random|RandomBool) "NewEnumerator1" "NewEnumerator0")) :Option%202 "NewEnumerator1")))
    (Utilities|FlowControl|Sequence
      (:then_0
        (Utilities|Time|SetTimerbyEvent (delegate Custom|AI_Hit) _returnvalue true))
      (:then_1
        (bind _output_get (Variables|Default|SetDefend (Math|Random|RandomBool)))
        (if _output_get
          (Utilities|FlowControl|Delay _returnvalue)
          (Variables|Default|SetDefend false)))
      (:then_2
        (if (Math|Random|RandomBool)
          (CallFunction|AIJump))))))

(event EventBeginPlay
  (|CallParentFunction)
  (Utilities|Time|SetTimerbyEvent (delegate Custom|AI_Hit) (Math|Random|RandomFloatinRange 0.5 1.5) true))

(event Collision|EventActorBeginOverlap
  (params (OtherActor :type Actor%20Object%20Reference)))

(event EventTick
  (params (DeltaSeconds :type Float%20%28single-precision%29))
  (|CallParentFunction DeltaSeconds)
  (if (Variables|Default|GetFinish)
    (CallFunction|Hit "NewEnumerator3")))

(fn ConstructionScript
  (|CallParentFunction))